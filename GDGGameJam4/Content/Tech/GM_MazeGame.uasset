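; Game mode for a local multiplayer maze game with monkey players, a bomb and a defuser.
; On BeginPlay it drops the bomb and defuser above two distinct random prop spawn points, creates an extra local player and restarts player 0 as BP_Monkey.
; After a short delay it gathers every controlled monkey and moves each to a random player spawn point, removing used points to avoid overlaps.
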(event `self.ReceiveBeginPlay`
  (`self.SpawnProps`)
  (`GameplayStatics.CreatePlayer` -1)
  (set `self.DefaultPawnClass` "/Game/Tech/BP_Monkey.BP_Monkey_C")
  (`self.RestartPlayer` (`GameplayStatics.GetPlayerController` 0))
  (`KismetSystemLibrary.Delay` 0.2)
  (`self.SetUpPlayers`))

(fn `SetUpPlayers`
  (for _index (range (`GameplayStatics.GetNumPlayerControllers`))
    (`KismetArrayLibrary.Array_Add` (`self.Players`) (cast `/Game/Tech/BP_Monkey` (`Controller.K2_GetPawn` (`GameplayStatics.GetPlayerController` _index)) :!pure true)))
  (`self.SpawnPlayers`))

(fn `SpawnPlayers`
  (locals (SpawnPositions :type "Array of Vector Structure") (indexReference :type Integer))
  (bind _spawnpositions (`local.SpawnPositions`))
  (bind _outactors (`GameplayStatics.GetAllActorsOfClass` "/Game/Tech/BP_SpawnPoint.BP_SpawnPoint_C"))
  (for _array_element _outactors
    (if (`|EnumEquality` (`/Game/Tech/BP_SpawnPoint.Type` _array_element) "NewEnumerator0")
      (`KismetArrayLibrary.Array_Add` (`local.SpawnPositions`) (`self.K2_GetActorLocation` _array_element))))
  (for _array_element_2 (`self.Players`)
    (bind _output_get (set `local.indexReference` (`.OutIndex` (`KismetArrayLibrary.Array_Random` _spawnpositions))))
    (`self.K2_SetActorLocation` _array_element_2 (`|GetArrayItem` (`local.SpawnPositions`) _output_get) false false)
    (`KismetArrayLibrary.Array_Remove` _spawnpositions _output_get)))

(fn `SpawnProps`
  (locals (Positions :type "Array of Vector Structure") (index :type Integer))
  (bind _outactors (`GameplayStatics.GetAllActorsOfClass` "/Game/Tech/BP_SpawnPoint.BP_SpawnPoint_C"))
  (for _array_element _outactors
    (if (`|EnumEquality` (`/Game/Tech/BP_SpawnPoint.Type` _array_element) "NewEnumerator1")
      (`KismetArrayLibrary.Array_Add` (`local.Positions`) (`self.K2_GetActorLocation` _array_element))))
  (bind _output_get (set `local.index` (`.OutIndex` (`KismetArrayLibrary.Array_Random` (`local.Positions`)))))
  (`|SpawnActorFromClass` "/Game/Tech/BP_Bomb.BP_Bomb_C" (`KismetMathLibrary.MakeTransform` (+ (`|GetArrayItem` (`local.Positions`) _output_get) (0.0 0.0 400.0))) "AdjustIfPossibleButAlwaysSpawn" "MultiplyWithRoot" null null)
  (`KismetArrayLibrary.Array_Remove` (`local.Positions`) (`local.index`))
  (set `local.index` (`.OutIndex` (`KismetArrayLibrary.Array_Random` (`local.Positions`))))
  (`|SpawnActorFromClass` "/Game/Tech/BP_Defuser.BP_Defuser_C" (`KismetMathLibrary.MakeTransform` (+ (`|GetArrayItem` (`local.Positions`) (`local.index`)) (0.0 0.0 400.0))) "AdjustIfPossibleButAlwaysSpawn" "MultiplyWithRoot" null null))

(fn `UserConstructionScript`)