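; Timed bomb actor for the maze game that ends the game on explosion unless a defuser reaches it first.
; After a short delay it starts a countdown sound and counts down on Tick, exploding through GM_MazeGame's GameEnd at zero.
; Overlapping a BP_Defuser stops the timer, snaps the defuser to a mesh socket with physics off, then destroys both and adds score.
; TogglePhysics switches mesh simulation, playing a pickup sound when disabled.
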(event `self.ReceiveBeginPlay`
  (`KismetSystemLibrary.Delay` 2.0)
  (set `self.run` true)
  (bind _returnvalue (`GameplayStatics.SpawnSound2D` "/Game/Audio/Sound-Cues/BombCountdown.BombCountdown" 1.0 1.0 0.0 null))
  (set `self.CountdownSound` _returnvalue))

(event `self.ReceiveActorBeginOverlap`
  (params (OtherActor :type "Actor Object Reference"))
  (if (== (`GameplayStatics.GetObjectClass` OtherActor) "/Game/Tech/Blueprints/BP_Defuser.BP_Defuser_C")
    (set `self.run` false)
    (bind _output_get (set `self.Other Actor` OtherActor))
    (`self.K2_AttachToComponent` (`self.Other Actor`) (`self.Mesh`) "defuseSocket" "SnapToTarget" "SnapToTarget" "SnapToTarget" true)
    (`self.TogglePhysics` false)
    (message `/Game/Tech/Blueprints/I_Item.TogglePhysics` (`self.Other Actor`) false)
    (`ActorComponent.SetActive` (`self.CountdownSound`) false false)
    (`KismetSystemLibrary.Delay` 1.0)
    (`GameplayStatics.PlaySound2D` "/Game/Audio/Sound-Cues/DefuseSound.DefuseSound" 1.0 1.0 0.0 null null)
    (`self.K2_DestroyActor` _output_get)
    (`self.K2_DestroyActor`)
    (bind _asgm_maze_game (cast `/Game/Tech/GameModes/GM_MazeGame` (`GameplayStatics.GetGameMode`)))
    (`/Game/Tech/GameModes/GM_MazeGame.UpdateScore` _asgm_maze_game 1)))

(event `self.ReceiveTick`
  (params (DeltaSeconds :type "Float (single-precision)"))
  (if (`self.run`)
    (bind _output_get (set `self.timeRemaining` (- (`self.timeRemaining`) DeltaSeconds)))
    (if (<= _output_get 0.0)
      (`self.K2_DestroyActor`)
      (`GameplayStatics.PlaySound2D` "/Game/Audio/Sound-Cues/BombExplosion.BombExplosion" 1.0 1.0 0.0 null null)
      (bind _asgm_maze_game (cast `/Game/Tech/GameModes/GM_MazeGame` (`GameplayStatics.GetGameMode`)))
      (`/Game/Tech/GameModes/GM_MazeGame.GameEnd` _asgm_maze_game))))

(event `/Game/Tech/Blueprints/I_Item.TogglePhysics`
  (params (condition :type Boolean))
  (`PrimitiveComponent.SetSimulatePhysics` (`self.Mesh`) condition)
  (if (== condition false)
    (`GameplayStatics.PlaySound2D` "/Game/Audio/Sound-Cues/BombPickup.BombPickup" 1.0 1.0 0.0 null null)))

(fn `UserConstructionScript`)