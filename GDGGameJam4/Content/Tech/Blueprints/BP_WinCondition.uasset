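; BP_WinCondition is an actor that checks whether a bomb and a defuser have both entered its overlap area.
; ActorBeginOverlap adds any BP_Bomb or BP_Defuser to the Objects array and calls WinCondition.
; WinCondition tallies both classes and, once each is present, destroys every stored actor.
; Objects is never pruned on overlap end or cleared, so actors that leave still count.
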(event `self.ReceiveActorBeginOverlap`
  (params (OtherActor :type "Actor Object Reference"))
  (if (or (== (`GameplayStatics.GetObjectClass` OtherActor) "/Game/Tech/Blueprints/BP_Bomb.BP_Bomb_C") (== (`GameplayStatics.GetObjectClass` OtherActor) "/Game/Tech/Blueprints/BP_Defuser.BP_Defuser_C"))
    (`KismetArrayLibrary.Array_Add` (`self.Objects`) OtherActor)
    (`self.WinCondition`)))

(fn `UserConstructionScript`)

(fn `WinCondition`
  (if (> (`KismetArrayLibrary.Array_Length` (`self.Objects`)) 1)
    (for _array_element (`self.Objects`)
      (bind _returnvalue (`GameplayStatics.GetObjectClass` _array_element))
      (if (== _returnvalue "/Game/Tech/Blueprints/BP_Bomb.BP_Bomb_C")
        (`/Engine/EditorBlueprintResources/StandardMacros.IncrementInt` (`self.bombCounter`))
        (elif (== _returnvalue "/Game/Tech/Blueprints/BP_Defuser.BP_Defuser_C")
          (`/Engine/EditorBlueprintResources/StandardMacros.IncrementInt` (`self.defuserCounter`)))))
    (if (and (> (`self.bombCounter`) 0) (> (`self.defuserCounter`) 0))
      (for _array_element_2 (`self.Objects`)
        (`self.K2_DestroyActor` _array_element_2)))))