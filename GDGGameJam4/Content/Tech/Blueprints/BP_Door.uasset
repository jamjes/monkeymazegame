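; BP_Door is a timed door that automatically alternates between open and closed states, starting with an unlock at BeginPlay.
; Tick counts down RemainingTime and toggles between Unlock and Lock when it expires.
; Each call instantly shifts the actor vertically, down to unlock and up to lock, then reloads the countdown from OpenTime or CloseTime.
; The TimerWidget visibility calls in both functions are disconnected and never run.
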(event `self.ReceiveBeginPlay`
  (`self.Unlock`))

(event `self.ReceiveTick`
  (params (DeltaSeconds :type "Float (single-precision)"))
  (bind _output_get (set `self.remainingTime` (- (`self.remainingTime`) DeltaSeconds)))
  (if (<= _output_get 0.0)
    (if (`self.isLocked`)
      (`self.Unlock`)
      (else
        (`self.Lock`)))))

(fn `Lock`
  (`self.K2_SetActorLocation` (+ (`self.K2_GetActorLocation`) (0.0 0.0 400.0)))
  (set `self.isLocked` true)
  (set `self.remainingTime` (`self.closeTime`)))

(fn `Unlock`
  (`self.K2_SetActorLocation` (+ (`self.K2_GetActorLocation`) (0.0 0.0 -400.0)))
  (set `self.isLocked` false)
  (set `self.remainingTime` (`self.openTime`)))

(fn `UserConstructionScript`)